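; Base actor for explosive environment objects that blow up from hard impacts or damage, hurting their surroundings.
; A mesh hit above an impulse threshold explodes it immediately, while damage through the vitality component ignites a fire and detonates after a delay.
; Death triggers a shorter delayed blast.
; The DoOnce-guarded explosion spawns effects and sound, applies environmental radial damage with falloff, then destroys the actor.
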(event `self.ObjectMesh.OnComponentHit`
  (params (HitComponent :type "PrimitiveComponent Object Reference") (OtherActor :type "Actor Object Reference") (OtherComp :type "PrimitiveComponent Object Reference") (NormalImpulse :type "Vector Structure") (Hit :type "HitResult Structure (by ref)"))
  (if (> (`KismetMathLibrary.VSize` NormalImpulse) (`self.ImpulseForceTreshord`))
    (`self.Explosion`)))

(event `Explosion`
  (bind _returnvalue (`self.K2_GetActorLocation`))
  (bind _damage (`self.Damage`))
  (bind _exploderadius (`self.ExplodeRadius`))
  (`/Engine/EditorBlueprintResources/StandardMacros.DoOnce` false
    (:`Completed`
      (`|ExecutionSequence`
        (:`then_0`
          (`|ExecutionSequence`
            (:`then_0`
              (`GameplayStatics.SpawnEmitterAtLocation` "/Game/M5VFXVOL2/Particles/Explosion/Fire_Exp_00.Fire_Exp_00" _returnvalue)
              (`GameplayStatics.SpawnSoundAtLocation` "/Game/StarterContent/Audio/Explosion02.Explosion02" _returnvalue (struct) 1.0 1.0 0.0 null null))
            (:`then_1`
              (`GameplayStatics.ApplyRadialDamageWithFalloff` :`BaseDamage` _damage :`MinimumDamage` (/ _damage 5.0) :`Origin` (`self.K2_GetActorLocation`) :`DamageInnerRadius` (/ _exploderadius 3.0) :`DamageOuterRadius` _exploderadius :`DamageFalloff` 1.0 :`DamageTypeClass` "/Engine/EngineDamageTypes/DmgTypeBP_Environmental.DmgTypeBP_Environmental_C" :`DamageCauser` null :`InstigatedByController` null :`DamagePreventionChannel` "ECC_GameTraceChannel2"))))
        (:`then_1`
          (`self.K2_DestroyActor`))))))

(event `self.BP_VitalityComponent.OnTakeDamage`
  (`ActorComponent.Activate` (`self.Fire`) true)
  (`KismetSystemLibrary.Delay` 3.0)
  (`self.Explosion`))

(event `self.BP_VitalityComponent.OnDead`
  (`KismetSystemLibrary.Delay` 1.0)
  (`self.Explosion`))

(fn `UserConstructionScript`)