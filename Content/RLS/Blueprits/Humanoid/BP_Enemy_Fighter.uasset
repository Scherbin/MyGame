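; BP_Enemy_Fighter is a humanoid melee enemy that extends its parent's attack logic with animated attacks and contact damage.
; StartAttack calls the parent, then plays a random attack montage, calling FinishAttack on completion or interruption.
; Any begin-overlap on the Mesh applies WeaponDamage as point damage, directed from the fighter toward the other actor, with no check on attack state or target.
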(event `PlayaAttackMontage`
  (`|PlayMontage` (`self.Mesh`) (`KismetArrayLibrary.Array_Random` (`self.AttackMontages`))
    (:`OnCompleted`
      _)
    (:`OnInterrupted`
      _))
  (`self.FinishAttack`))

(event `self.Mesh.OnComponentBeginOverlap`
  (params (OverlappedComponent :type "PrimitiveComponent Object Reference") (OtherActor :type "Actor Object Reference") (OtherComp :type "PrimitiveComponent Object Reference") (OtherBodyIndex :type Integer) (bFromSweep :type Boolean) (SweepResult :type "HitResult Structure (by ref)"))
  (`GameplayStatics.ApplyPointDamage` OtherActor (`self.WeaponDamage`) (`KismetMathLibrary.Normal` (- (`self.K2_GetActorLocation` OtherActor) (`self.K2_GetActorLocation`))) SweepResult))

(fn `StartAttack`
  (`parent.StartAttack`)
  (`self.PlayaAttackMontage`))

(fn `UserConstructionScript`
  (`parent.UserConstructionScript`))