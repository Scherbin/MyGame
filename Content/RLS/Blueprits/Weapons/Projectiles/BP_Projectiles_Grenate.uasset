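; BP_Projectiles_Grenate is a grenade projectile that explodes two seconds after BeginPlay, or earlier when its Sphere hits an actor tagged Enemy.
; Explosion spawns fire particles and sound, then applies falloff radial damage with BP_DT_Granate, using inner and outer radii derived from ExplodeRadius.
; It also draws a debug sphere at the inner radius, then destroys the actor.
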(event `self.ReceiveBeginPlay`
  (`KismetSystemLibrary.Delay` 2.0)
  (`self.Explosion`))

(event `self.Sphere.OnComponentHit`
  (params (HitComponent :type "PrimitiveComponent Object Reference") (OtherActor :type "Actor Object Reference") (OtherComp :type "PrimitiveComponent Object Reference") (NormalImpulse :type "Vector Structure") (Hit :type "HitResult Structure (by ref)"))
  (if (`self.ActorHasTag` OtherActor "Enemy")
    (`self.Explosion`)))

(event `Explosion`
  (bind _returnvalue (`self.K2_GetActorLocation`))
  (bind _damage (`self.Damage`))
  (bind _exploderadius (`self.ExplodeRadius`))
  (`|ExecutionSequence`
    (:`then_0`
      (`|ExecutionSequence`
        (:`then_0`
          (`GameplayStatics.SpawnEmitterAtLocation` "/Game/M5VFXVOL2/Particles/Explosion/Fire_Exp_00.Fire_Exp_00" _returnvalue)
          (`GameplayStatics.SpawnSoundAtLocation` "/Game/StarterContent/Audio/Explosion02.Explosion02" _returnvalue (struct) 1.0 1.0 0.0 null null))
        (:`then_1`
          (`KismetSystemLibrary.DrawDebugSphere` (`self.K2_GetActorLocation`) (`self.ExplodeRadius`) 0 (struct :`R` 0.649306 :`G` 0.009018 :`B` 0.009018 :`A` 1.0))
          (`GameplayStatics.ApplyRadialDamageWithFalloff` :`BaseDamage` _damage :`MinimumDamage` (/ _damage 5.0) :`Origin` (`self.K2_GetActorLocation`) :`DamageInnerRadius` _exploderadius :`DamageOuterRadius` (* _exploderadius 3.0) :`DamageFalloff` 1.0 :`DamageTypeClass` "/Game/RLS/Damage/BP_DT_Granate.BP_DT_Granate_C" :`DamageCauser` null :`InstigatedByController` null))))
    (:`then_1`
      (`self.K2_DestroyActor`))))

(fn `UserConstructionScript`
  (`parent.UserConstructionScript`))