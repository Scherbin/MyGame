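; BP_W2 is a child weapon Blueprint with automatic hitscan primary fire and an alternate grenade launcher.
; Primary fire uses a looping timer to spend ammo and trace shots until the attack finishes or ammo runs out.
; Alt fire spawns a grenade aimed at a camera sphere-trace point, without checking the ammo-spend result.
; Both modes extend parent shot checks and activate their own sound and muzzle effects.
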(event `StartBurs`
  (`self.OneShot`)
  (bind _returnvalue (`KismetSystemLibrary.K2_SetTimerDelegate` (delegate `OneShot`) 0.1 true))
  (set `self.Burst_TH` _returnvalue))

(event `OneShot`
  (bind _result (`self.TrySpendAmo` true))
  (if _result
    (`self.MakeTraceShot` true)
    (`ActorComponent.Activate` (`self.ShotSound_Main`) true)
    (`ActorComponent.Activate` (`self.Muzzle_Main`) true)
    (else
      (`self.Finish_Burst`))))

(event `Finish_Burst`
  (`KismetSystemLibrary.K2_ClearAndInvalidateTimerHandle` (`self.Burst_TH`)))

(event `LauncheGrenade`
  (bind _returnvalue_location (`KismetMathLibrary.BreakTransform` (`SceneComponent.K2_GetComponentToWorld` (`self.dir_Alt`))))
  (`self.TrySpendAmo` false)
  (if true
    (`|SpawnActorFromClass` "/Game/RLS/Blueprits/Weapons/Projectiles/BP_Projectiles_Grenate.BP_Projectiles_Grenate_C" (`KismetMathLibrary.MakeTransform` _returnvalue_location (`self.GetGrenateRotation`)) "AdjustIfPossibleButDontSpawnIfColliding" "OverrideRootScale" null null)
    (`ActorComponent.Activate` (`self.Muzzle_Alt`) true)
    (`ActorComponent.Activate` (`self.ShotSound_Alt`) true)))

(fn `FinishAttackMain`
  (`parent.FinishAttackMain`)
  (`self.Finish_Burst`))

(fn `GetGrenateRotation`
  (returns (Rotation :type "Rotator Structure"))
  (locals (TargetPoint :type "Vector Structure"))
  (bind _returnvalue (`GameplayStatics.GetPlayerCameraManager` 0))
  (bind _returnvalue_2 (`PlayerCameraManager.GetCameraLocation` _returnvalue))
  (bind _outhit (`KismetSystemLibrary.SphereTraceSingle` _returnvalue_2 (+ _returnvalue_2 (* (`self.GetActorForwardVector` _returnvalue) 5000.0)) 5.0 "TraceTypeQuery1"))
  (bind (_bblockinghit _binitialoverlap _time _distance _location _impactpoint _normal _impactnormal _physmat _hitactor _hitcomponent _hitbonename _hititem _elementindex _faceindex _tracestart _traceend) (`GameplayStatics.BreakHitResult` _outhit))
  (bind _output_get (set `local.TargetPoint` (select `bool` _bblockinghit :`false` _traceend :`true` _location)))
  (return (`KismetMathLibrary.FindLookAtRotation` (`SceneComponent.K2_GetComponentLocation` (`self.dir_Alt`)) _output_get)))

(fn `TryMakeShot_Alt`
  (returns (Result :type Boolean))
  (bind _result (`parent.TryMakeShot_Alt`))
  (if _result
    (`self.LauncheGrenade`)
    (return true)
    (else
      (return false))))

(fn `TryMakeShot_Main`
  (returns (Result :type Boolean))
  (bind _result (`parent.TryMakeShot_Main`))
  (if _result
    (`self.StartBurs`)
    (return true)
    (else
      (return false))))

(fn `UserConstructionScript`
  (`parent.UserConstructionScript`))