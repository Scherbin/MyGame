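; Weapon Blueprint with a rifle-style main fire and a shotgun-like volley alt fire, both built on parent shot checks.
; Main fire spends ammo, fires one trace with sound and muzzle effects, then resets its ready flag after a delay.
; Alt fire spends alt ammo and runs a looping timer of multi-pellet trace volleys, widening scatter each volley until the volley count clears the timer.
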(event `MakeRifleShot`
  (bind _result (`self.TrySpendAmo` true))
  (if _result
    (set `self.IsMainShotReady` false)
    (`self.MakeTraceShot` true)
    (`ActorComponent.Activate` (`self.ShotSound_Main`) true)
    (`ActorComponent.Activate` (`self.Muzzle_Main`) true)
    (`KismetSystemLibrary.Delay` 0.5)
    (set `self.IsMainShotReady` true)))

(event `MakeAltShot`
  (if (`self.IsAltShotReady`)
    (bind _result (`self.TrySpendAmo` false))
    (if _result
      (set `self.IsAltShotReady` false)
      (set `self.CurrentVolleyIndex` 0)
      (bind _returnvalue (`KismetSystemLibrary.K2_SetTimerDelegate` (`|CreateDelegate` :!event `MakeVolley`) (`self.VolleyTime`) true))
      (set `self.ValleyTH` _returnvalue)
      (`self.MakeVolley`)
      (`ActorComponent.Activate` (`self.ShotSound_Alt`) true)
      (`ActorComponent.Activate` (`self.Muzzle_Alt`) true)
      (`KismetSystemLibrary.Delay` 1.0)
      (set `self.IsAltShotReady` true))))

(event `MakeVolley`
  (`|ExecutionSequence`
    (:`then_0`
      (set `self.ScatterAlt` (+ (`self.AltScatterBase`) (* (`self.CurrentVolleyIndex`) (`self.AltDeltaScatter`))))
      (for _ (range 1 (+ (`self.PelletAmount`) 1))
        (`self.MakeTraceShot` false)))
    (:`then_1`
      (bind _result (`/Engine/EditorBlueprintResources/StandardMacros.IncrementInt` (`self.CurrentVolleyIndex`))
        (:`  `
          (if (>= _result (`self.VolleyAmount`))
            (`KismetSystemLibrary.K2_ClearAndInvalidateTimerHandle` (`self.ValleyTH`))))))))

(fn `TryMakeShot_Alt`
  (returns (Result :type Boolean))
  (bind _result (`parent.TryMakeShot_Alt`))
  (if _result
    (`self.MakeAltShot`)
    (return true)
    (else
      (return false))))

(fn `TryMakeShot_Main`
  (returns (Result :type Boolean))
  (bind _result (`parent.TryMakeShot_Main`))
  (if _result
    (`self.MakeRifleShot`)
    (return true)
    (else
      (return false))))

(fn `UserConstructionScript`
  (`parent.UserConstructionScript`))