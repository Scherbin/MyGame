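; Base weapon Blueprint providing main and alt fire, ammo tracking and reloading.
; Shots sphere-trace from the player camera within a random scatter cone, draw a debug line from the fire-direction component and apply point damage.
; Per-mode settings drive each shot, though range selection is crossed: main uses RangeAlt, alt uses RangeMain.
; Ammo spending and reloading from the reserve broadcast OnAmmoChanged; FinishAttackMain is an empty stub.
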(event `self.ReceiveBeginPlay`
  (set `self.Ammo` (`self.AmmoInClip`)))

(fn `FinishAttackMain`)

(fn `MakeTraceShot`
  (params (`Main?` :type Boolean))
  (bind _returnvalue (`GameplayStatics.GetPlayerCameraManager` 0))
  (bind _returnvalue_2 (`PlayerCameraManager.GetCameraLocation` _returnvalue))
  (bind _outhit (`KismetSystemLibrary.SphereTraceSingle` _returnvalue_2 (+ _returnvalue_2 (* (`KismetMathLibrary.RandomUnitVectorInConeInDegrees` (`self.GetActorForwardVector` _returnvalue) (select `bool` (`local.Main?`) :`false` (`self.Scatter_Alt`) :`true` (`self.Scatter_Main`))) (select `bool` (`local.Main?`) :`false` (`self.Range_Main`) :`true` (`self.Range_Alt`)))) 3.0 "TraceTypeQuery1" true))
  (bind (_bblockinghit _binitialoverlap _time _distance _location _impactpoint _normal _impactnormal _physmat _hitactor _hitcomponent _hitbonename _hititem _elementindex _faceindex _tracestart _traceend) (`GameplayStatics.BreakHitResult` _outhit))
  (`KismetSystemLibrary.DrawDebugLine` (`SceneComponent.K2_GetComponentLocation` (select `bool` (`local.Main?`) :`false` (`self.dir_Alt`) :`true` (`self.Dir_Main`))) (select `bool` _bblockinghit :`false` _traceend :`true` _impactpoint) (struct :`G` 0.06332 :`B` 1.0 :`A` 1.0) 0.3 1.0)
  (bind (_bblockinghit_2 _binitialoverlap_2 _time_2 _distance_2 _location_2 _impactpoint_2 _normal_2 _impactnormal_2 _physmat_2 _hitactor_2 _hitcomponent_2 _hitbonename_2 _hititem_2 _elementindex_2 _faceindex_2 _tracestart_2 _traceend_2) (`GameplayStatics.BreakHitResult` _outhit))
  (`GameplayStatics.ApplyPointDamage` _hitactor_2 (select `bool` (`local.Main?`) :`false` (`self.Damage_Alt`) :`true` (`self.Damage_Main`)) (- _traceend_2 _tracestart_2) _outhit null null (select `bool` (`local.Main?`) :`false` (`self.DamageType_Alt`) :`true` (`self.damageType_Main`) :!type "DamageType Class Reference")))

(fn `ReloadWeapon`
  (if (> (`self.Total_Ammo`) 0)
    (`|ExecutionSequence`
      (:`then_0`
        (set `self.Total_Ammo` (+ (`self.Ammo`) (`self.Total_Ammo`)))
        (set `self.Ammo` 0)
        (if (>= (`self.Total_Ammo`) (`self.AmmoInClip`))
          (set `self.Total_Ammo` (- (`self.Total_Ammo`) (`self.AmmoInClip`)))
          (set `self.Ammo` (`self.AmmoInClip`))
          (else
            (set `self.Ammo` (`self.Total_Ammo`))
            (set `self.Total_Ammo` 0))))
      (:`then_1`
        (`self.OnAmmoChanged` (`self.Ammo`) (`self.Total_Ammo`) (`self.SpecAmmo`))))))

(fn `TryMakeShot_Alt`
  (returns (Result :type Boolean))
  (return (> (`self.SpecAmmo`) 0)))

(fn `TryMakeShot_Main`
  (returns (Result :type Boolean))
  (return (> (`self.Ammo`) 0)))

(fn `TrySpendAmo`
  (params (`Main?` :type Boolean))
  (returns (Result :type Boolean))
  (if (> (select `bool` (`local.Main?`) :`false` (`self.SpecAmmo`) :`true` (`self.Ammo`)) 0)
    (`/Engine/EditorBlueprintResources/StandardMacros.DecrementInt` (select `bool` (`local.Main?`) :`false` (`self.SpecAmmo`) :`true` (`self.Ammo`))
      (:`  `
        (`self.OnAmmoChanged` (`self.Ammo`) (`self.Total_Ammo`) (`self.SpecAmmo`))
        (return true)))
    (else
      (return false))))

(fn `UserConstructionScript`)