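; BP_Lever is an interactable lever that toggles between two positions and signals the change through a turn-on dispatcher.
; Each interaction flips IsUp, then plays or reverses the Move_TL timeline.
; The timeline interpolates the Moveble component's relative pitch to swing the lever, and on finishing calls OnTurnOn with the inverse of IsUp.
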(event `self.BP_Interactabal.OnStartInteract`
  (bind _output_get (set `self.IsUp` (not (`self.IsUp`))))
  (if _output_get
    (bind (_direction _newtrack_0) (`Timeline|Move_TL` :!via `Reverse` :!label _label)
      (:`Update`
        (`SceneComponent.K2_SetRelativeRotation` (`self.Moveble`) (`KismetMathLibrary.MakeRotator` 0.0 (`KismetMathLibrary.Lerp` 0.0 -120.0 _newtrack_0)) false false))
      (:`Finished`
        (`self.OnTurnOn` (not (`self.IsUp`)))))
    (else
      (goto _label))))

(fn `UserConstructionScript`
  (`parent.UserConstructionScript`))