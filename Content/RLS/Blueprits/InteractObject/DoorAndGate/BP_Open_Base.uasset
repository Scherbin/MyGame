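; BP_Open_Base is a door and gate base actor that opens and closes in response to linked activators.
; On BeginPlay it binds to the toggle and turn-on events of each valid entry in Activators.
; Toggle flips the open state through TurnOn, which ignores unchanged states and plays or reverses a timeline.
; The timeline lerps OpenComp's relative transform toward the MovebleOffset transform, without sweeping.
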(event `self.ReceiveBeginPlay`
  (for _array_element (`self.Activators`)
    (`/Engine/EditorBlueprintResources/StandardMacros.IsValid` _array_element
      (:`Is Valid`
        (add `/Game/RLS/Blueprits/InteractObject/InreractableActivators/BP_InteractleActivator_Base.OnTugle` _array_element (delegate `Toggle`))
        (add `/Game/RLS/Blueprits/InteractObject/InreractableActivators/BP_InteractleActivator_Base.OnTurnOn` _array_element (`|CreateDelegate` :!event `TurnOn`))))))

(event `Toggle`
  (`self.TurnOn` (not (`self.IsTutnOn?`))))

(event `TurnOn`
  (params (`On/Off` :type Boolean))
  (if (!= `On/Off` (`self.IsTutnOn?`))
    (bind _output_get (set `self.IsTutnOn?` `On/Off`))
    (if _output_get
      (bind (_direction _newtrack_0) (`Timeline|MoveOpen_TL` :!label _label)
        (:`Update`
          (`SceneComponent.K2_SetRelativeTransform` (`self.openComp`) (`KismetMathLibrary.TLerp` (`KismetMathLibrary.MakeTransform` (0.0 0.0 0.0)) (`self.MovebleOffset`) _newtrack_0) false false)))
      (else
        (goto _label :!via `Reverse`)))))

(fn `UserConstructionScript`)