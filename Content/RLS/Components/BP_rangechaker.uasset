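; BP_rangechaker is a component that detects when player 0's camera moves into or out of range of its owning actor.
; Every tick it stores the camera-to-owner distance in Cathdistance and compares it to ReliseDistance, the single threshold for both directions.
; The IsCatch flag latches the state, so the OnCatch and OnRelise dispatchers fire only on each crossing.
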(event `self.ReceiveTick`
  (params (DeltaSeconds :type "Float (single-precision)"))
  (set `self.Cathdistance` (`KismetMathLibrary.VSize` (- (`PlayerCameraManager.GetCameraLocation` (`GameplayStatics.GetPlayerCameraManager` 0)) (`Actor.K2_GetActorLocation` (`self.GetOwner`)))))
  (if (`self.IsCatch`)
    (if (> (`self.Cathdistance`) (`self.ReliseDistance`))
      (set `self.IsCatch` false)
      (`self.OnRelise`))
    (elif (< (`self.Cathdistance`) (`self.ReliseDistance`))
      (set `self.IsCatch` true)
      (`self.OnCatch`))))