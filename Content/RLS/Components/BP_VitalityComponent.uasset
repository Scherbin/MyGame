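; Actor component that manages its owner's health, damage, healing and death, broadcasting HP change, damage and death events.
; It binds to the owner's point and radial damage events, routing both into ApplyDamage, which marks death below half a point.
; Damage restarts an optional delayed, looping regen timer that heals a percentage of max HP until full.
; ApplyDamage casts the damage type, but its ResistanceMap scaling is disconnected and never runs.
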(event `self.ReceiveBeginPlay`
  (bind _returnvalue (`self.GetOwner`))
  (add `Actor.OnTakePointDamage` _returnvalue (delegate `PointDamage`))
  (add `Actor.OnTakeRadialDamage` _returnvalue (delegate `Radialdamage`))
  (bind _output_get (set `self.CurrentHP` (`self.TotalHP`)))
  (`KismetSystemLibrary.Delay` 0.0)
  (`self.OnHPChanged` _output_get (`self.TotalHP`)))

(event `Radialdamage`
  (params (DamagedActor :type "Actor Object Reference") (Damage :type "Float (double-precision)") (DamageType :type "DamageType Object Reference") (Origin :type "Vector Structure") (HitInfo :type "HitResult Structure") (InstigatedBy :type "Controller Object Reference") (DamageCauser :type "Actor Object Reference"))
  (`self.ApplyDamage` Damage DamageType))

(event `PointDamage`
  (params (DamagedActor :type "Actor Object Reference") (Damage :type "Float (double-precision)") (InstigatedBy :type "Controller Object Reference") (HitLocation :type "Vector Structure") (FHitComponent :type "PrimitiveComponent Object Reference") (BoneName :type Name) (ShotFromDirection :type "Vector Structure") (DamageType :type "DamageType Object Reference") (DamageCauser :type "Actor Object Reference"))
  (`self.ApplyDamage` Damage DamageType))

(event `ApplyRegen`
  (if (`self.HaveRegen`)
    (`KismetSystemLibrary.K2_ClearAndInvalidateTimerHandle` (`self.RegenTH`))
    (bind _returnvalue (`KismetSystemLibrary.K2_SetTimerDelegate` (delegate `RegetHP`) (`self.RegenTickDelay`) true (`self.RegenStartDelay`)))
    (set `self.RegenTH` _returnvalue)))

(event `RegetHP`
  (`self.ApplyHeal` (* (* (/ (`self.RegenPercentperScond`) 100.0) (`self.TotalHP`)) (`self.RegenTickDelay`)))
  (if (>= (`self.CurrentHP`) (`self.TotalHP`))
    (`KismetSystemLibrary.K2_ClearAndInvalidateTimerHandle` (`self.RegenTH`))))

(fn `ApplyDamage`
  (params (BaseDamage :type "Float (double-precision)") (DamageType :type "DamageType Object Reference"))
  (locals (ActualDamage :type "Float (double-precision)"))
  (set `local.ActualDamage` BaseDamage)
  (if (`self.IsAlive`)
    (`|ExecutionSequence`
      (:`then_0`
        (bind _asbp_damage_type_base (cast `/Game/RLS/Damage/BP_DamageType_Base` (`local.DamageType`))))
      (:`then_1`
        (if (> (`local.ActualDamage`) 0.0)
          (`self.ApplyRegen`)
          (bind _output_get (set `self.CurrentHP` (- (`self.CurrentHP`) (`local.ActualDamage`))))
          (`self.OnHPChanged` _output_get (`self.TotalHP`))
          (`self.OnTakeDamage`)))
      (:`then_2`
        (if (< (`self.CurrentHP`) 0.5)
          (set `self.CurrentHP` 0.0)
          (set `self.IsAlive` false)
          (`self.OnDead`))))))

(fn `ApplyHeal`
  (params (HealAmount :type "Float (double-precision)"))
  (set `self.CurrentHP` (`KismetMathLibrary.FClamp` (+ HealAmount (`self.CurrentHP`)) 0.0 (`self.TotalHP`)))
  (`self.OnHPChanged` (`self.CurrentHP`) (`self.TotalHP`)))