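; BP_ImpactEffect is an actor that plays a surface-specific impact effect at its own location and rotation.
; On BeginPlay it reads the physical material surface type from its Hit variable to select a particle emitter, with Default and Metal sharing one template.
; It also spawns a short-lived decal selected by the same surface type, but every decal material slot is empty.
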(event `self.ReceiveBeginPlay`
  (bind _surfacetype (`PhysicalMaterial.SurfaceType` (`.PhysMat` (`GameplayStatics.BreakHitResult` (`self.Hit`)))))
  (`GameplayStatics.SpawnEmitterAtLocation` (select `EPhysicalSurface` _surfacetype :`SurfaceType_Default` "/Game/Realistic_Starter_VFX_Pack_Vol2/Particles/Hit/P_Default.P_Default" :`SurfaceType1` "/Game/Realistic_Starter_VFX_Pack_Vol2/Particles/Hit/P_Default.P_Default" :`SurfaceType2` "/Game/Realistic_Starter_VFX_Pack_Vol2/Particles/Hit/P_Wood.P_Wood" :`SurfaceType3` "/Game/Realistic_Starter_VFX_Pack_Vol2/Particles/Hit/P_Ice.P_Ice" :`SurfaceType4` "/Game/Realistic_Starter_VFX_Pack_Vol2/Particles/Hit/P_Asphalt.P_Asphalt" :`SurfaceType5` "/Game/Realistic_Starter_VFX_Pack_Vol2/Particles/Blood/P_Blood_Splat_Cone.P_Blood_Splat_Cone" :!type "ParticleSystem Object Reference") (`self.K2_GetActorLocation`) (`self.K2_GetActorRotation`))
  (`GameplayStatics.SpawnDecalAtLocation` (select `EPhysicalSurface` _surfacetype :!type "MaterialInterface Object Reference") (2.0 40.0 4.0) (`self.K2_GetActorLocation`) (`self.K2_GetActorRotation`) 10.0))

(fn `UserConstructionScript`)